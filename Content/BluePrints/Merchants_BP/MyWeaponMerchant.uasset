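; Weapon merchant actor that shows an interaction prompt and a shop screen to the player.
; BeginPlay adds both widgets to the viewport, and Tick sets their visibility from the overlapping and interacting flags, which are not set in this graph.
; AssignWeaponRowsandColoumns creates a weapon entry widget, places it in the merchant's inventory grid and copies the weapon's ID, name, description, damage and cost into it.
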(event EventBeginPlay
  (bind _returnvalue (Game|GetPlayerController 0))
  (bind _returnvalue_2 (UserInterface|CreateWidget "/Game/BluePrints/UI_BP/InteractionMessage.InteractionMessage_C" _returnvalue))
  (bind _output_get (Variables|Default|SetInteractionMessage _returnvalue_2))
  (UserInterface|Viewport|AddtoViewport _output_get 0)
  (bind _returnvalue_3 (UserInterface|CreateWidget "/Game/BluePrints/UI_BP/WeaponMerchant.WeaponMerchant_C" _returnvalue))
  (bind _output_get_2 (Variables|Default|SetMerchantScreen _returnvalue_3))
  (UserInterface|Viewport|AddtoViewport _output_get_2 0))

(event Collision|EventActorBeginOverlap
  (params (OtherActor :type Actor%20Object%20Reference)))

(event EventTick
  (params (DeltaSeconds :type Float%20%28single-precision%29))
  (bind _merchantscreen (Variables|Default|GetMerchantScreen))
  (bind _interactionmessage (Variables|Default|GetInteractionMessage))
  (if (Variables|Default|GetbIsCharacterOverlapping)
    (Widget|SetVisibility _interactionmessage "Visible")
    (if (Variables|Default|GetbIsCharacterInteracting)
      (Widget|SetVisibility _merchantscreen "Visible")
      (Widget|SetVisibility (Variables|Default|GetInteractionMessage) "Hidden")
      (else
        (Widget|SetVisibility _merchantscreen "Hidden" :!label _label)))
    (else
      (Widget|SetVisibility _interactionmessage "Hidden")
      (goto _label))))

(event EventAssignWeaponRowsandColoumns
  (bind _returnvalue (UserInterface|CreateWidget "/Game/BluePrints/UI_BP/WeaponInMerchant.WeaponInMerchant_C"))
  (bind _returnvalue_2 (Class|GridPanel|AddChildtoGrid (Variables|/Game/BluePrints/UI_BP/WeaponMerchant.WeaponMerchant_C|GetMerchantInventory (Variables|Default|GetMerchantScreen)) _returnvalue (Variables|Default|GetRow) (Variables|Default|GetColoumn)))
  (Layout|BorderSlot|SetPadding _returnvalue_2 (Utilities|Struct|MakeMargin 0.0 1e+01 15.0 0.0) :!class /Script/UMG.GridSlot)
  (Variables|/Game/BluePrints/UI_BP/WeaponInMerchant.WeaponInMerchant_C|SetWeaponId _returnvalue (Variables|Default|GetWeaponID))
  (Variables|/Game/BluePrints/UI_BP/WeaponInMerchant.WeaponInMerchant_C|SetWeaponDamage _returnvalue (Variables|Default|GetWeaponDamage))
  (Variables|/Game/BluePrints/UI_BP/WeaponInMerchant.WeaponInMerchant_C|SetWeaponDescription _returnvalue (Variables|Default|GetWeaponDescription))
  (Variables|/Game/BluePrints/UI_BP/WeaponInMerchant.WeaponInMerchant_C|SetWeaponName _returnvalue (Variables|Default|GetWeaponName))
  (Variables|/Game/BluePrints/UI_BP/WeaponInMerchant.WeaponInMerchant_C|SetWeaponCost _returnvalue (Variables|Default|GetWeaponCost)))

(fn ConstructionScript)