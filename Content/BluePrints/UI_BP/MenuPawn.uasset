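; Pawn for the Dunception title screen that drives the menu UI.
; On BeginPlay it creates the MenuUI title widget, adds it to the viewport and shows the mouse cursor.
; Any key press hides the title and press-any-key text, then creates the main menu widget, guarded by a flag so it is only created once.
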(event EventBeginPlay
  (bind _returnvalue (Game|GetPlayerController 0))
  (bind _returnvalue_2 (UserInterface|CreateWidget "/Game/BluePrints/UI_BP/MenuUI.MenuUI_C" _returnvalue))
  (UserInterface|Viewport|AddtoViewport _returnvalue_2 0)
  (Variables|/Script/Engine.PlayerController|SetbShowMouseCursor _returnvalue true)
  (Variables|Default|SetIsMainMenuCreated false))

(event Collision|EventActorBeginOverlap
  (params (OtherActor :type Actor%20Object%20Reference)))

(event EventTick
  (params (DeltaSeconds :type Float%20%28single-precision%29)))

(event Input|KeyboardEvents|AnyKey
  (params (Key :type Key%20Structure :default "None"))
  (:Pressed
    (Widget|SetVisibility (Variables|/Game/BluePrints/UI_BP/MenuUI.MenuUI_C|GetAnyKeyText (stale EventBeginPlay _returnvalue_2)) "Hidden")
    (Widget|SetVisibility (Variables|/Game/BluePrints/UI_BP/MenuUI.MenuUI_C|GetDunception (stale EventBeginPlay _returnvalue_2)) "Hidden")
    (if (not (Variables|Default|GetIsMainMenuCreated))
      (Variables|Default|SetIsMainMenuCreated true)
      (bind _returnvalue (UserInterface|CreateWidget "/Game/BluePrints/UI_BP/MainMenu.MainMenu_C" (Game|GetPlayerController 0)))
      (UserInterface|Viewport|AddtoViewport _returnvalue 0))))

(fn ConstructionScript)